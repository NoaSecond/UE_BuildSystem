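; Actor component for a building system that places, rotates and deletes BP_PlaceableBlueprint actors, switching PC_BuildSystem HUDs by mode.
; In build mode, Tick spawns the controller's selected class once until reset, then grid-snaps it to a camera trace; inputs rotate or place it.
; In delete mode, a camera trace tints targets red, and Delete destroys them.
; Save and spawn functions store placed actors as class and transform maps and recreate them.
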(event `InputAction|Unload`
  (params (Key :type "Key Structure"))
  ;[1 1 1] Inputs
  ;;[1 1 1] Unload
  (:`Pressed`
    (`self.ToggleBuildMode` false)))

(event `self.ReceiveBeginPlay`
  ;[1 1 1] Init
  (bind _aspc_build_system (cast `/Game/BuildSystem/PC_BuildSystem` (`GameplayStatics.GetPlayerController` 0)))
  (set `self.PCBuildSystem_REF` _aspc_build_system))

(event `ToggleDeleteMode`
  (params (IsDeleting :type Boolean))
  ;[1 1 1] Toggle modes
  (bind _output_get (set `self.IsDeleting` IsDeleting))
  (if _output_get
    (set `self.IsBuilding` false)
    (`/Game/BuildSystem/PC_BuildSystem.SwitchToDeleteHUD` (`self.PCBuildSystem_REF`))))

(event `ToggleBuildMode`
  (params (IsBuilding :type Boolean))
  ;[1 1 1] Toggle modes
  (bind _output_get (set `self.IsBuilding` IsBuilding))
  (if _output_get
    (set `self.IsDeleting` false)
    (`/Game/BuildSystem/PC_BuildSystem.SwitchToBuildHUD` (`self.PCBuildSystem_REF`))
    (else
      (bind _buildblueprint (`self.BuildBlueprint`)
        (:`then`
          (`Actor.K2_DestroyActor` _buildblueprint))
        (:`else`)))))

(event `InputAxisKey|MouseWheelAxis`
  (params (AxisValue :type "Float (single-precision)"))
  ;[1 1 1] Inputs
  ;;[1 1 1] Blueprint rotation
  (if (`self.IsBuilding`)
    (bind _buildblueprint (`self.BuildBlueprint`)
      (:`then`
        (`Actor.K2_SetActorRotation` _buildblueprint (`KismetMathLibrary.ComposeRotators` (`Actor.K2_GetActorRotation` (`self.BuildBlueprint`)) (`KismetMathLibrary.MakeRotator` 0.0 0.0 (* AxisValue (`self.RotationSensivity`)))) false))
      (:`else`))))

(event `InputAction|PlaceBuildBlueprint`
  (params (Key :type "Key Structure"))
  ;[1 1 1] Inputs
  ;;[1 1 1] Place BP
  (:`Pressed`
    (bind _buildblueprint (`self.BuildBlueprint`)
      (:`then`
        (`/Game/BuildSystem/PlaceableBlueprints/BP_PlaceableBlueprint.Placed` _buildblueprint (`self.Latest_Rotation`) (`self.Latest_Scale`)))
      (:`else`))))

(event `self.ReceiveTick`
  (params (DeltaSeconds :type "Float (single-precision)"))
  (bind _returnvalue_location (`KismetMathLibrary.BreakTransform` (`Actor.GetTransform` (`self.ParentActorRef`))))
  (if (`self.IsBuilding`)
    ;[1 1 1] Building
    (`|ExecutionSequence`
      (:`then_0`
        (`/Engine/EditorBlueprintResources/StandardMacros.DoOnce` false :!label _label
          (:`Completed`
            (set `self.Latest_Rotation` (`KismetMathLibrary.MakeVector` (.x (stale `ResetBuild` Rotation)) (.y (stale `ResetBuild` Rotation)) (.z (stale `ResetBuild` Rotation))))
            (set `self.Latest_Scale` (stale `ResetBuild` Scale))
            (bind _returnvalue (`|SpawnActorFromClass` (`/Game/BuildSystem/PC_BuildSystem.BuildBlueprint_Class` (`self.PCBuildSystem_REF`)) (`KismetMathLibrary.MakeTransform` _returnvalue_location (`KismetMathLibrary.MakeRotator` (.x (stale `ResetBuild` Rotation)) (.y (stale `ResetBuild` Rotation)) (.z (stale `ResetBuild` Rotation))) (stale `ResetBuild` Scale)) "Undefined" "OverrideRootScale" null null))
            (set `self.BuildBlueprint` _returnvalue))))
      (:`then_1`
        (bind _location (`self.BuildTrace`))
        (bind _buildblueprint (`self.BuildBlueprint`)
          (:`then`
            (`Actor.K2_SetActorLocation` _buildblueprint (`KismetMathLibrary.Vector_SnappedToGrid` _location (`self.SnapGridSize`)) false false))
          (:`else`))))
    (else
      ;[1 1 1] Deleting
      (if (`self.IsDeleting`)
        (bind _hitactor (`self.DeleteTrace`))
        (bind _asbp_placeable_blueprint (cast `/Game/BuildSystem/PlaceableBlueprints/BP_PlaceableBlueprint` _hitactor))
        (`/Game/BuildSystem/PlaceableBlueprints/BP_PlaceableBlueprint.ChangeMaterial` _asbp_placeable_blueprint "/Game/BuildSystem/Materials/M_Preview_Red.M_Preview_Red")))))

(event `ResetBuild`
  (params (Rotation :type "Vector Structure") (Scale :type "Vector Structure"))
  ;[1 1 1] Building
  (goto _label :!via `Reset`))

(event `InputAction|DeleteMode`
  (params (Key :type "Key Structure"))
  ;[1 1 1] Inputs
  ;;[1 1 1] Switch in delete mode
  (:`Pressed`
    (`self.ToggleBuildMode` false)
    (`self.ToggleDeleteMode` true)))

(event `InputAction|Delete`
  (params (Key :type "Key Structure"))
  ;[1 1 1] Inputs
  ;;[1 1 1] Delete PB
  (:`Pressed`
    (bind _hitactor (`self.DeleteTrace`))
    (bind _asbp_placeable_blueprint (cast `/Game/BuildSystem/PlaceableBlueprints/BP_PlaceableBlueprint` _hitactor))
    (`/Game/BuildSystem/PlaceableBlueprints/BP_PlaceableBlueprint.Destroyed` _asbp_placeable_blueprint)))

(fn `BuildTrace`
  (returns (Location :type "Vector Structure"))
  (locals (BuildHitDistance :type "Float (single-precision)" :default 5000.0))
  (bind _returnvalue (`GameplayStatics.GetPlayerCameraManager` 0))
  (bind _returnvalue_2 (`PlayerCameraManager.GetCameraLocation` _returnvalue))
  (bind _outhit (`KismetSystemLibrary.LineTraceSingle` _returnvalue_2 (+ _returnvalue_2 (* (`KismetMathLibrary.GetForwardVector` (`PlayerCameraManager.GetCameraRotation` _returnvalue)) (`local.BuildHitDistance`))) "TraceTypeQuery1"))
  (return (`.Location` (`GameplayStatics.BreakHitResult` _outhit))))

(fn `DeleteTrace`
  (returns (HitActor :type "Actor Object Reference"))
  (locals (DeleteHitDistance :type "Float (double-precision)" :default 500.0))
  (bind _returnvalue (`GameplayStatics.GetPlayerCameraManager` 0))
  (bind _returnvalue_2 (`PlayerCameraManager.GetCameraLocation` _returnvalue))
  (bind _outhit (`KismetSystemLibrary.LineTraceSingle` :`Start` _returnvalue_2 :`End` (+ _returnvalue_2 (* (`KismetMathLibrary.GetForwardVector` (`PlayerCameraManager.GetCameraRotation` _returnvalue)) (`local.DeleteHitDistance`))) :`TraceChannel` "TraceTypeQuery1" :`DrawDebugType` "ForOneFrame"))
  (return (`.HitActor` (`GameplayStatics.BreakHitResult` _outhit))))

(fn `SavePBList`
  (returns (PBList_Class :type "Map of Integer to /Game/BuildSystem/PlaceableBlueprints/BP_PlaceableBlueprint Class Reference") (PBList_Transform :type "Map of Integer to Transform Structure") (ReturnValue :type "EventReply Structure"))
  (`BlueprintMapLibrary.Map_Clear` (`self.PBList_Class`))
  (`BlueprintMapLibrary.Map_Clear` (`self.PBList_Transform`))
  (bind _outactors (`GameplayStatics.GetAllActorsOfClass` "/Game/BuildSystem/PlaceableBlueprints/BP_PlaceableBlueprint.BP_PlaceableBlueprint_C"))
  (for (_array_element _array_index) _outactors
    (`BlueprintMapLibrary.Map_Add` (`self.PBList_Class`) _array_index (`GameplayStatics.GetObjectClass` _array_element))
    (`BlueprintMapLibrary.Map_Add` (`self.PBList_Transform`) _array_index (`Actor.GetTransform` _array_element)))
  (return (`self.PBList_Class`) (`self.PBList_Transform`) (`WidgetBlueprintLibrary.Handled`)))

(fn `SpawnPBList`
  (params (PBList_Class :type "Map of Integer to /Game/BuildSystem/PlaceableBlueprints/BP_PlaceableBlueprint Class Reference") (PBList_Transform :type "Map of Integer to Transform Structure"))
  (returns (ReturnValue :type "EventReply Structure"))
  (bind _keys (`BlueprintMapLibrary.Map_Keys` PBList_Class))
  (for (_ _array_index) _keys
    (bind _values (`BlueprintMapLibrary.Map_Values` PBList_Class))
    (bind _values_2 (`BlueprintMapLibrary.Map_Values` PBList_Transform))
    (bind _output (`|GetArrayItem` _values_2 _array_index))
    (bind _returnvalue (`|SpawnActorFromClass` (`|GetArrayItem` _values _array_index) _output "Undefined" "OverrideRootScale" null null))
    (`/Game/BuildSystem/PlaceableBlueprints/BP_PlaceableBlueprint.Placed` _returnvalue (`KismetMathLibrary.Conv_RotatorToVector` (.rotation _output)) (.scale _output)))
  (return (`WidgetBlueprintLibrary.Handled`)))