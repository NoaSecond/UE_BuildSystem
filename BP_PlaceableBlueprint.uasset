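; Placeable actor for a build system, acting as both the placement preview and the placed object.
; On BeginPlay it caches the mesh's first material, swaps to a green preview material and disables collision.
; Placed restores material and collision, then calls ResetBuild on the player character's ACBuildSystem through PC_BuildSystem, passing rotation and scale.
; Other events swap the material, add world rotation or set scale.
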(event `self.ReceiveBeginPlay`
  (set `self.InitialMaterial` (`PrimitiveComponent.GetMaterial` (`self.StaticMesh`) 0))
  (`self.ChangeMaterial` "/Game/BuildSystem/M_Preview_Green.M_Preview_Green")
  (`PrimitiveComponent.SetCollisionEnabled` (`self.StaticMesh`) "NoCollision"))

(event `Placed`
  (params (Rotation :type "Vector Structure") (Scale :type "Vector Structure"))
  (`self.ResetMaterial`)
  (`PrimitiveComponent.SetCollisionEnabled` (`self.StaticMesh`) "QueryAndPhysics")
  (bind _aspc_build_system (cast `/Game/BuildSystem/PC_BuildSystem` (`GameplayStatics.GetPlayerController` 0)))
  (`/Game/BuildSystem/AC_BuildSystem.ResetBuild` (`/Game/ThirdPerson/Blueprints/BP_ThirdPersonCharacter.AC_BuildSystem` (`/Game/BuildSystem/PC_BuildSystem.PlayerCharacterRef` _aspc_build_system)) Rotation Scale))

(event `ChangeMaterial`
  (params (NewMaterial :type "MaterialInterface Object Reference"))
  (`PrimitiveComponent.SetMaterial` (`self.StaticMesh`) 0 NewMaterial))

(event `ResetMaterial`
  (`self.ChangeMaterial` (`self.InitialMaterial`)))

(event `EditRotation`
  (params (Rotation :type "Vector Structure"))
  (`self.K2_AddActorWorldRotation` self (`KismetMathLibrary.MakeRotator` Rotation_X Rotation_Y Rotation_Z) false false))

(event `EditScale`
  (params (Scale :type "Vector Structure"))
  (`self.SetActorScale3D` self Scale))

(fn `UserConstructionScript`)