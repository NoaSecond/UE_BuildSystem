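; Player controller for the build system, linking the first-person character's build component to its UI and loading the saved map.
; On BeginPlay it hands character and camera references to that component, creates HUD and inventory widgets, and respawns saved pieces from the save slot named in the game mode's options.
; FlipFlop toggles swap HUD and inventory or show the cursor, while events switch the HUD between build, delete and idle modes.
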(event `self.ReceiveBeginPlay`
  (bind _optionsstring (`GameModeBase.OptionsString` (`GameplayStatics.GetGameMode`)))
  ;[1 1 1] Init
  (set `self.CurrentLevelName` (`GameplayStatics.ParseOption` _optionsstring "SlotName"))
  (set `self.CurrentLevelAuthor` (`GameplayStatics.ParseOption` _optionsstring "SlotName"))
  (bind _asbp_first_person_character (cast `/Game/BuildSystem/FPSEditingCharacter/BP_FirstPersonCharacter` (`GameplayStatics.GetPlayerCharacter` 0)))
  (set `self.PlayerCharacterRef` _asbp_first_person_character)
  (bind _ac_buildsystem (`/Game/BuildSystem/FPSEditingCharacter/BP_FirstPersonCharacter.AC_BuildSystem` _asbp_first_person_character))
  (set `/Game/BuildSystem/AC_BuildSystem.ParentActorRef` (`self.PlayerCharacterRef`) _ac_buildsystem)
  (set `/Game/BuildSystem/AC_BuildSystem.CameraRef` (`/Game/BuildSystem/FPSEditingCharacter/BP_FirstPersonCharacter.FirstPersonCamera` _asbp_first_person_character) _ac_buildsystem)
  (`|ExecutionSequence`
    (:`then_0`
      (bind _returnvalue (`|CreateWidget` "/Game/BuildSystem/UI/UI_BS_HUD.UI_BS_HUD_C"))
      (bind _output_get (set `self.UI_BS_HUD_REF` _returnvalue))
      (`UserWidget.AddToViewport` _output_get 0)
      (`self.LoadAndSpawnPBList`)
      (`WidgetBlueprintLibrary.SetInputMode_GameOnly` self))
    (:`then_1`
      (bind _returnvalue_2 (`|CreateWidget` "/Game/BuildSystem/UI/UI_BS_Inventory.UI_BS_Inventory_C"))
      (set `self.UI_BS_Invetory_REF` _returnvalue_2))))

(event `ToggleBSInventory`
  (bind _ui_bs_hud_ref (`self.UI_BS_HUD_REF`))
  (bind _ui_bs_invetory_ref (`self.UI_BS_Invetory_REF`))
  ;[1 1 1] Toggle Inventory
  (`/Engine/EditorBlueprintResources/StandardMacros.FlipFlop`
    (:`A`
      (`UserWidget.AddToViewport` _ui_bs_invetory_ref 0)
      (`Widget.RemoveFromParent` _ui_bs_hud_ref)
      (`WidgetBlueprintLibrary.SetInputMode_GameAndUIEx` self null)
      (set `self.bShowMouseCursor` true))
    (:`B`
      (`Widget.RemoveFromParent` _ui_bs_invetory_ref)
      (`UserWidget.AddToViewport` _ui_bs_hud_ref 0)
      (`WidgetBlueprintLibrary.SetInputMode_GameOnly` self)
      (set `self.bShowMouseCursor` false))))

(event `SwitchToDeleteHUD`
  ;[1 1 1] Switch HUD Mode
  (`/Game/BuildSystem/UI/UI_BS_HUD.ShowDeleteHUD` (`self.UI_BS_HUD_REF`)))

(event `InputAction|ToggleMouseCursor`
  (params (Key :type "Key Structure"))
  ;[1 1 1] Toggle mouse cursor
  (:`Pressed`
    (`/Engine/EditorBlueprintResources/StandardMacros.FlipFlop` :!label _label
      (:`A`
        (`WidgetBlueprintLibrary.SetInputMode_GameAndUIEx` self null)
        (set `self.bShowMouseCursor` true))
      (:`B`
        (`WidgetBlueprintLibrary.SetInputMode_GameOnly` self)
        (set `self.bShowMouseCursor` false)))))

(event `SwitchToBuildHUD`
  ;[1 1 1] Switch HUD Mode
  (`/Game/BuildSystem/UI/UI_BS_HUD.ShowBuildHUD` (`self.UI_BS_HUD_REF`)))

(event `ToggleMouseCursor`
  ;[1 1 1] Toggle mouse cursor
  (goto _label))

(event `SwitchToIdleHUD`
  ;[1 1 1] Switch HUD Mode
  (`/Game/BuildSystem/UI/UI_BS_HUD.ShowIdleHUD` (`self.UI_BS_HUD_REF`)))

(event `LoadAndSpawnPBList`
  ;[1 1 1] Load & Spawn PBList
  (bind _returnvalue (`GameplayStatics.LoadGameFromSlot` (`self.CurrentLevelName`)))
  (bind _assg_bs_map_data (cast `/Game/BuildSystem/SG_BS_MapData` _returnvalue))
  (bind _pb_list_class (`/Game/BuildSystem/SG_BS_MapData.PB_List_Class` _assg_bs_map_data))
  (if (`BlueprintMapLibrary.Map_IsNotEmpty` _pb_list_class)
    (`/Game/BuildSystem/AC_BuildSystem.SpawnPBList` (`/Game/BuildSystem/FPSEditingCharacter/BP_FirstPersonCharacter.AC_BuildSystem` (`self.PlayerCharacterRef`)) _pb_list_class (`/Game/BuildSystem/SG_BS_MapData.PB_List_Transform` _assg_bs_map_data))))

(fn `UserConstructionScript`)